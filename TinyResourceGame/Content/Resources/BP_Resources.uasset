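; BP_Resources is a harvestable resource actor that holds a count of remaining units.
; Harvest returns the requested amount, capped at UnitsLeft, and destroys the actor when UnitsLeft is zero or below.
; The subtraction is reversed (Collected minus UnitsLeft), so the result is never positive and any harvest destroys the actor.
; The event graph and construction script are empty.
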(fn `Harvest`
  (params (DesiredAmount :type Integer))
  (returns (CollectedAmount :type Integer))
  (locals (Collected :type Integer))
  ;[1 1 1] Determine collected amount
  (bind _output_get (set `local.Collected` (`KismetMathLibrary.Min` DesiredAmount (`self.UnitsLeft`))))
  ;[1 1 1] Subtract Collected Units
  (bind _output_get_2 (set `self.UnitsLeft` (- _output_get (`self.UnitsLeft`))))
  ;[1 1 1] Check has depleted
  (if (<= _output_get_2 0)
    (`self.K2_DestroyActor`))
  (return (`local.Collected`)))

(fn `UserConstructionScript`)