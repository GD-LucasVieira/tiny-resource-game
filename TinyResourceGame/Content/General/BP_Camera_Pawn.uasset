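; Camera pawn that shows the cursor and provides movement, yaw rotation and spring-arm zoom.
; Tick polls Enhanced Input values, applying key-driven local move, strafe and rotation scaled by delta time.
; Middle mouse drives a drag move, though its forward and right offsets are multiplied rather than added, cancelling out.
; Otherwise right mouse rotates, and with neither held, zoom changes arm length within min/max limits.
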(event `self.ReceiveBeginPlay`
  (set `PlayerController.bShowMouseCursor` true (`GameplayStatics.GetPlayerController` 0)))

(event `self.ReceiveTick`
  (params (DeltaSeconds :type "Float (single-precision)"))
  (bind (_returnvalue_x _returnvalue_y) (`KismetMathLibrary.BreakVector2D` (`|GetInputActionValue`)))
  (bind _maxcameraspeed (`self.MaxCameraSpeed`))
  (bind _springarm (`self.SpringArm`))
  (bind _returnvalue (+ (* (`|GetInputActionValue`) (`self.CameraZoomSpeed`)) (`SpringArmComponent.TargetArmLength` _springarm)))
  ;[1 1 1] Move by Keys
  (`self.K2_AddActorLocalOffset` (* (`KismetMathLibrary.GetForwardVector` (struct)) (`|GetInputActionValue`) (`self.MaxCameraSpeed`) DeltaSeconds))
  ;[1 1 1] Strafe by Keys
  (`self.K2_AddActorLocalOffset` (* (`KismetMathLibrary.GetRightVector` (struct)) (`|GetInputActionValue`) (`self.MaxCameraSpeed`) DeltaSeconds))
  ;[1 1 1] Rotate by Keys
  (`self.K2_AddActorLocalRotation` (`KismetMathLibrary.MakeRotator` 0.0 0.0 (* (`|GetInputActionValue`) DeltaSeconds (`self.CameraRotationSpeed`))))
  ;[1 1 1] Move By Mouse
  (if (`PlayerController.IsInputKeyDown` (`GameplayStatics.GetPlayerController` 0) "MiddleMouseButton")
    (`self.K2_AddActorLocalOffset` (* (* (`KismetMathLibrary.GetForwardVector` (struct)) _maxcameraspeed _returnvalue_y DeltaSeconds -1.0) (* (`KismetMathLibrary.GetRightVector` (struct)) _returnvalue_x _maxcameraspeed DeltaSeconds -1.0)))
    (else
      ;[1 1 1] Rotate Camera By Mouse
      (if (`PlayerController.IsInputKeyDown` (`GameplayStatics.GetPlayerController` 0) "RightMouseButton")
        (`self.K2_AddActorLocalRotation` (`KismetMathLibrary.MakeRotator` 0.0 0.0 (* _returnvalue_x (`self.CameraRotationSpeed`) DeltaSeconds)))
        (else
          ;[1 1 1] Zoom
          (if (and (<= _returnvalue (`self.MaxArmLength`)) (>= _returnvalue (`self.MinArmLenght`)))
            (set `SpringArmComponent.TargetArmLength` _returnvalue _springarm)))))))

(fn `UserConstructionScript`)